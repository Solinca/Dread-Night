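; BP_MapDisplay is a map display with a spring-arm camera that supports scrolling, rotating, zooming and recentering on a player marker.
; Input events set desired location, rotation and zoom, which Tick interpolates before updating the spring arm's transform and length.
; Locations use normalized -1 to 1 coordinates, scaled up during interpolation to avoid snapping.
; Scrolling follows map rotation, with speed and clamped bounds varying by zoom.
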(event Custom|Set%20Map%20Location
  (params (New%20Map%20Location :type Vector%202D%20Structure) (Move%20Instantly :type Boolean))
  ;[0 0 0 0.5] Set the camera location on the map.
  ;;[0 0 0 0.5] Save the desired location
  (bind _output_get (Variables|Scrolling|SetDesired%20Map%20Location New%20Map%20Location))
  ;;[0 0 0 0.5] If we should move instantly, match the desired location and update the camera
  (if Move%20Instantly
    (bind _output_get_2 (Variables|Scrolling|SetDesired%20Map%20Location (CallFunction|ClampMapLocation _output_get)))
    (Variables|Scrolling|SetCurrent%20Map%20Location _output_get_2)
    (CallFunction|UpdateCamera)))

(event Custom|Set%20Zoom%20Level
  (params (Zoom%20Level :type Float%20%28double-precision%29))
  ;[0 0 0 0.5] Force zoom to the desired level (0-1)
  (Variables|Scrolling|SetDesired%20Map%20Zoom (Math|Float|Clamp(Float) Zoom%20Level)))

(event Custom|Scroll%20Map
  (params (Scroll%20Delta :type Vector%202D%20Structure))
  ;[0 0 0 0.5] Scroll the map
  ;;[0 0 0 0.5] Update the map scroll coordinates
  (CallFunction|SetMapLocation (+ (Class|KismetMathLibrary|GetRotated2D (* Scroll%20Delta (Math|Float|MapRangeClamped (Variables|Scrolling|GetCurrent%20Map%20Zoom) 0.0 1.0 (Variables|Scrolling|GetMin%20Scroll%20Speed) (Variables|Scrolling|GetMax%20Scroll%20Speed))) (+ (Variables|Rotation|GetCurrent%20Map%20Rotation) 9e+01)) (Variables|Scrolling|GetDesired%20Map%20Location)) false))

(event Custom|Rotate%20Map
  (params (Rotation%20Delta :type Float%20%28double-precision%29))
  ;[0 0 0 0.5] Rotate the map
  (Variables|Rotation|SetDesired%20Map%20Rotation (+ (* Rotation%20Delta (Variables|Rotation|GetMap%20Rotation%20Multiplier)) (Variables|Rotation|GetDesired%20Map%20Rotation))))

(event Custom|Zoom%20Map
  (params (Zoom%20Delta :type Float%20%28double-precision%29))
  ;[0 0 0 0.5] Scroll the map by the desired delta
  (CallFunction|SetZoomLevel (+ Zoom%20Delta (Variables|Scrolling|GetDesired%20Map%20Zoom))))

(event Custom|Update%20Camera
  (bind _current_map_location (Variables|Scrolling|GetCurrent%20Map%20Location))
  (bind _springarm (Variables|Default|GetSpringArm))
  (bind _map_size (Variables|MapDimensions|GetMap%20Size))
  (bind _returnvalue (* _current_map_location _map_size))
  ;[0 0 0 0.5] Updates the map's camera by setting the spring arm location
  ;;[0 0 0 0.5] Set the spring map transform to scroll and rotate
  (Transformation|SetRelativeLocationAndRotation _springarm (Math|Vector|MakeVector (.x _returnvalue) (.y _returnvalue) 5e+02) (Math|Rotator|MakeRotator 0.0 -8e+01 (Variables|Rotation|GetCurrent%20Map%20Rotation)) false false)
  ;;[0 0 0 0.5] Set the spring arm length to zoom
  (Variables|/Script/Engine.SpringArmComponent|SetTargetArmLength _springarm (Math|Float|MapRangeClamped (Variables|Scrolling|GetCurrent%20Map%20Zoom) 0.0 1.0 (Variables|MapDimensions|GetCamera%20Distance%20Min) (Variables|MapDimensions|GetCamera%20Distance%20Max))))

(event Custom|Set%20Player%20Coordinates
  (params (Coords :type Vector%202D%20Structure) (Camera%20Heading :type Float%20%28double-precision%29))
  ;[0 0 0 0.5] Initialize the map with the player coordinates
  ;;[0 0 0 0.5] Reset the map so it zooms in on the player location
  (Variables|Scrolling|SetCurrent%20Map%20Zoom 1.0)
  (Variables|Scrolling|SetDesired%20Map%20Zoom 0.0)
  ;;[0 0 0 0.5] Save the player location so we can revert back to it later
  (bind _output_get (Variables|Scrolling|SetPlayer%20Location Coords))
  (CallFunction|SetMapLocation _output_get true)
  ;;[0 0 0 0.5] Place the player marker on the map
  (Transformation|SetRelativeLocationAndRotation (Variables|Default|GetPlayerLocation) (Math|Vector|MakeVector (.x (* _output_get (Variables|MapDimensions|GetMap%20Size))) (.y (* _output_get (Variables|MapDimensions|GetMap%20Size))) 5e+02) (Math|Rotator|MakeRotator 0.0 0.0 Camera%20Heading) false false))

(event Custom|Recenter%20Map%20on%20Player
  ;[0 0 0 0.5] Center the map back to the cached player location
  (CallFunction|SetMapLocation (Variables|Scrolling|GetPlayer%20Location) false))

(event EventBeginPlay
  ;[0 0 0 0.5] Add the Map ISM
  (AddComponent|AddInstancedStaticMeshComponent false))

(event EventTick
  (params (DeltaSeconds :type Float%20%28single-precision%29))
  (bind _returnvalue (Math|Float|MakeLiteralFloat 1e+02))
  ;[0 0 0 0.5] Update
  ;;[0 0 0 0.5] Animate the Zoom
  (Variables|Scrolling|SetCurrent%20Map%20Zoom (Math|Interpolation|FInterpTo (Variables|Scrolling|GetCurrent%20Map%20Zoom) (Variables|Scrolling|GetDesired%20Map%20Zoom) DeltaSeconds (Variables|Zoom|GetZoom%20Update%20Speed)))
  ;;[0 0 0 0.5] Clamp the desired map location to the bounds corresponding to our zoom level. More zoom out means we can't get as close to the edge.
  (Variables|Scrolling|SetDesired%20Map%20Location (CallFunction|ClampMapLocation (Variables|Scrolling|GetDesired%20Map%20Location)))
  ;;[0 0 0 0.5] Animate the map location. Since we're working on normalized -1 to 1 space, the change may become so small that InterpTo causes a snap, so we animate at a scale 100 times larger.
  (Variables|Scrolling|SetCurrent%20Map%20Location (CallFunction|ClampMapLocation (/ (Class|KismetMathLibrary|Vector2DInterpto (* (Variables|Scrolling|GetCurrent%20Map%20Location) _returnvalue) (* (Variables|Scrolling|GetDesired%20Map%20Location) _returnvalue) DeltaSeconds (Variables|Scrolling|GetScroll%20Update%20Speed)) _returnvalue)))
  ;;[0 0 0 0.5] Animate the map rotation
  (Variables|Rotation|SetCurrent%20Map%20Rotation (Math|Interpolation|FInterpTo (Variables|Rotation|GetCurrent%20Map%20Rotation) (Variables|Rotation|GetDesired%20Map%20Rotation) DeltaSeconds (Variables|Rotation|GetRotation%20Update%20Speed)))
  ;;[0 0 0 0.5] Update the camera
  (CallFunction|UpdateCamera))

(fn ConstructionScript)

(fn ClampMapLocation
  (params (In%20Location :type Vector%202D%20Structure))
  (bind _min_zoom_scroll_range (Variables|Zoom|GetMin%20Zoom%20Scroll%20Range))
  (bind _max_zoom_scroll_range (Variables|Zoom|GetMax%20Zoom%20Scroll%20Range))
  (bind _current_map_zoom (Variables|Scrolling|GetCurrent%20Map%20Zoom))
  (bind _returnvalue (Math|Float|MapRangeClamped _current_map_zoom 0.0 1.0 _max_zoom_scroll_range _min_zoom_scroll_range))
  (return (Class|KismetMathLibrary|ClampAxes2D (/ (Class|KismetMathLibrary|ClampAxes2D (* In%20Location (Variables|MapDimensions|GetMap%20Size)) (* _returnvalue -1.0) _returnvalue) (Variables|MapDimensions|GetMap%20Size)) -1.0 1.0)))